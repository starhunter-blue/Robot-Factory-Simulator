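; Robot NPC eye actor that plays expressions: happy, blink, small, sad and left/right angry.
; The construction script creates a dynamic instance of M_RobotEyes, and each event steps its EyePhaseNr scalar through timed frames like a flipbook, some also sliding the mesh vertically.
; CurrentlyChangingExpression drops requests while one plays; most expressions return to neutral, but angry ones hold their last frame.
; AdvanceEye is a helper that increments the current phase.
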(event Custom|Event%20PlayHappy
  (bind _material (Variables|Default|GetMaterial))
  (bind _material_2 (Variables|Default|GetMaterial))
  (if (not (Variables|Default|GetCurrentlyChangingExpression))
    (CallFunction|EventSettoNeutral)
    (Variables|Default|SetCurrentlyChangingExpression true)
    (Components|MoveComponentTo (Variables|Default|GetStaticMesh) "-10.000000, 0,15.000000" "0,-180.000000, 0" false false 0.15 false)
    (Rendering|Material|SetScalarParameterValue _material_2 "EyePhaseNr" 21.0 :!class /Script/Engine.MaterialInstanceDynamic)
    (Utilities|FlowControl|Delay (Variables|Default|GetBetweenAnimationDelay))
    (Rendering|Material|SetScalarParameterValue _material_2 "EyePhaseNr" 22.0 :!class /Script/Engine.MaterialInstanceDynamic)
    (Utilities|FlowControl|Delay (Variables|Default|GetBetweenAnimationDelay))
    (Rendering|Material|SetScalarParameterValue _material_2 "EyePhaseNr" 25.0 :!class /Script/Engine.MaterialInstanceDynamic)
    (Utilities|FlowControl|Delay 1.5)
    (Components|MoveComponentTo (Variables|Default|GetStaticMesh) "-10.000000, 0,0.000000" "0,-180.000000, 0" false false 0.15 false)
    (Rendering|Material|SetScalarParameterValue _material "EyePhaseNr" 22.0 :!class /Script/Engine.MaterialInstanceDynamic)
    (Utilities|FlowControl|Delay (Variables|Default|GetBetweenAnimationDelay))
    (Rendering|Material|SetScalarParameterValue _material "EyePhaseNr" 21.0 :!class /Script/Engine.MaterialInstanceDynamic)
    (Utilities|FlowControl|Delay (Variables|Default|GetBetweenAnimationDelay))
    (Rendering|Material|SetScalarParameterValue _material "EyePhaseNr" 21.0 :!class /Script/Engine.MaterialInstanceDynamic)
    (Utilities|FlowControl|Delay (Variables|Default|GetBetweenAnimationDelay))
    (Rendering|Material|SetScalarParameterValue _material "EyePhaseNr" 0.0 :!class /Script/Engine.MaterialInstanceDynamic)
    (Variables|Default|SetCurrentlyChangingExpression false)))

(event Custom|Event%20Set%20to%20Neutral
  (Rendering|Material|SetScalarParameterValue (Variables|Default|GetMaterial) "EyePhaseNr" 0.0 :!class /Script/Engine.MaterialInstanceDynamic)
  (Components|MoveComponentTo (Variables|Default|GetStaticMesh) "-10.000000, 0,0.000000" "0,-180.000000, 0" false false 0.15 false))

(event Custom|Event%20Blink
  (if (not (Variables|Default|GetCurrentlyChangingExpression))
    (CallFunction|EventSettoNeutral)
    (Variables|Default|SetCurrentlyChangingExpression true)
    (Rendering|Material|SetScalarParameterValue (Variables|Default|GetMaterial) "EyePhaseNr" 13.0 :!class /Script/Engine.MaterialInstanceDynamic)
    (Utilities|FlowControl|Delay (Variables|Default|GetBetweenAnimationDelay))
    (Rendering|Material|SetScalarParameterValue (Variables|Default|GetMaterial) "EyePhaseNr" 18.0 :!class /Script/Engine.MaterialInstanceDynamic)
    (Utilities|FlowControl|Delay (Variables|Default|GetBetweenAnimationDelay))
    (Rendering|Material|SetScalarParameterValue (Variables|Default|GetMaterial) "EyePhaseNr" 19.0 :!class /Script/Engine.MaterialInstanceDynamic)
    (Utilities|FlowControl|Delay (Variables|Default|GetBetweenAnimationDelay))
    (Rendering|Material|SetScalarParameterValue (Variables|Default|GetMaterial) "EyePhaseNr" 26.0 :!class /Script/Engine.MaterialInstanceDynamic)
    (Utilities|FlowControl|Delay (Variables|Default|GetBetweenAnimationDelay))
    (Rendering|Material|SetScalarParameterValue (Variables|Default|GetMaterial) "EyePhaseNr" 7.0 :!class /Script/Engine.MaterialInstanceDynamic)
    (Utilities|FlowControl|Delay (Variables|Default|GetBetweenAnimationDelay))
    (Rendering|Material|SetScalarParameterValue (Variables|Default|GetMaterial) "EyePhaseNr" 26.0 :!class /Script/Engine.MaterialInstanceDynamic)
    (Utilities|FlowControl|Delay (Variables|Default|GetBetweenAnimationDelay))
    (Rendering|Material|SetScalarParameterValue (Variables|Default|GetMaterial) "EyePhaseNr" 19.0 :!class /Script/Engine.MaterialInstanceDynamic)
    (Utilities|FlowControl|Delay (Variables|Default|GetBetweenAnimationDelay))
    (Rendering|Material|SetScalarParameterValue (Variables|Default|GetMaterial) "EyePhaseNr" 18.0 :!class /Script/Engine.MaterialInstanceDynamic)
    (Utilities|FlowControl|Delay (Variables|Default|GetBetweenAnimationDelay))
    (Rendering|Material|SetScalarParameterValue (Variables|Default|GetMaterial) "EyePhaseNr" 13.0 :!class /Script/Engine.MaterialInstanceDynamic)
    (CallFunction|EventSettoNeutral)
    (Variables|Default|SetCurrentlyChangingExpression false)))

(event Custom|Event%20Small%20Eyes
  (if (not (Variables|Default|GetCurrentlyChangingExpression))
    (CallFunction|EventSettoNeutral)
    (Variables|Default|SetCurrentlyChangingExpression true)
    (Rendering|Material|SetScalarParameterValue (Variables|Default|GetMaterial) "EyePhaseNr" 1e+01 :!class /Script/Engine.MaterialInstanceDynamic)
    (Utilities|FlowControl|Delay (Variables|Default|GetBetweenAnimationDelay))
    (Rendering|Material|SetScalarParameterValue (Variables|Default|GetMaterial) "EyePhaseNr" 11.0 :!class /Script/Engine.MaterialInstanceDynamic)
    (Utilities|FlowControl|Delay (Variables|Default|GetBetweenAnimationDelay))
    (Rendering|Material|SetScalarParameterValue (Variables|Default|GetMaterial) "EyePhaseNr" 12.0 :!class /Script/Engine.MaterialInstanceDynamic)
    (Utilities|FlowControl|Delay 2.0)
    (Rendering|Material|SetScalarParameterValue (Variables|Default|GetMaterial) "EyePhaseNr" 11.0 :!class /Script/Engine.MaterialInstanceDynamic)
    (Utilities|FlowControl|Delay (Variables|Default|GetBetweenAnimationDelay))
    (Rendering|Material|SetScalarParameterValue (Variables|Default|GetMaterial) "EyePhaseNr" 1e+01 :!class /Script/Engine.MaterialInstanceDynamic)
    (Utilities|FlowControl|Delay (Variables|Default|GetBetweenAnimationDelay))
    (CallFunction|EventSettoNeutral)
    (Variables|Default|SetCurrentlyChangingExpression false)))

(event Custom|Event%20Angry%20Eye%20L
  (if (not (Variables|Default|GetCurrentlyChangingExpression))
    (CallFunction|EventSettoNeutral)
    (Components|MoveComponentTo (Variables|Default|GetStaticMesh) "-10.000000, 0,10.000000" "0,-180.000000, 0" false false 0.15 false)
    (Variables|Default|SetCurrentlyChangingExpression true)
    (Rendering|Material|SetScalarParameterValue (Variables|Default|GetMaterial) "EyePhaseNr" 1.0 :!class /Script/Engine.MaterialInstanceDynamic)
    (Utilities|FlowControl|Delay (Variables|Default|GetBetweenAnimationDelay))
    (Rendering|Material|SetScalarParameterValue (Variables|Default|GetMaterial) "EyePhaseNr" 2.0 :!class /Script/Engine.MaterialInstanceDynamic)
    (Utilities|FlowControl|Delay (Variables|Default|GetBetweenAnimationDelay))
    (Rendering|Material|SetScalarParameterValue (Variables|Default|GetMaterial) "EyePhaseNr" 3.0 :!class /Script/Engine.MaterialInstanceDynamic)
    (Utilities|FlowControl|Delay (Variables|Default|GetBetweenAnimationDelay))
    (Rendering|Material|SetScalarParameterValue (Variables|Default|GetMaterial) "EyePhaseNr" 4.0 :!class /Script/Engine.MaterialInstanceDynamic)
    (Utilities|FlowControl|Delay 1e+01)
    (Variables|Default|SetCurrentlyChangingExpression false)))

(event Custom|Event%20Angry%20Eye%20R
  (if (not (Variables|Default|GetCurrentlyChangingExpression))
    (CallFunction|EventSettoNeutral)
    (Components|MoveComponentTo (Variables|Default|GetStaticMesh) "-10.000000, 0,10.000000" "0,-180.000000, 0" false false 0.15 false)
    (Variables|Default|SetCurrentlyChangingExpression true)
    (Rendering|Material|SetScalarParameterValue (Variables|Default|GetMaterial) "EyePhaseNr" 5.0 :!class /Script/Engine.MaterialInstanceDynamic)
    (Utilities|FlowControl|Delay (Variables|Default|GetBetweenAnimationDelay))
    (Rendering|Material|SetScalarParameterValue (Variables|Default|GetMaterial) "EyePhaseNr" 6.0 :!class /Script/Engine.MaterialInstanceDynamic)
    (Utilities|FlowControl|Delay (Variables|Default|GetBetweenAnimationDelay))
    (Rendering|Material|SetScalarParameterValue (Variables|Default|GetMaterial) "EyePhaseNr" 8.0 :!class /Script/Engine.MaterialInstanceDynamic)
    (Utilities|FlowControl|Delay (Variables|Default|GetBetweenAnimationDelay))
    (Rendering|Material|SetScalarParameterValue (Variables|Default|GetMaterial) "EyePhaseNr" 9.0 :!class /Script/Engine.MaterialInstanceDynamic)
    (Utilities|FlowControl|Delay 1e+01)
    (Variables|Default|SetCurrentlyChangingExpression false)))

(event Custom|Event%20Sad%20Eyes
  (if (not (Variables|Default|GetCurrentlyChangingExpression))
    (CallFunction|EventSettoNeutral)
    (Variables|Default|SetCurrentlyChangingExpression true)
    (Components|MoveComponentTo (Variables|Default|GetStaticMesh) "-10.000000, 0,-5.000000" "0,-180.000000, 0" false false 0.15 false)
    (Rendering|Material|SetScalarParameterValue (Variables|Default|GetMaterial) "EyePhaseNr" 3e+01 :!class /Script/Engine.MaterialInstanceDynamic)
    (Utilities|FlowControl|Delay (Variables|Default|GetBetweenAnimationDelay))
    (Rendering|Material|SetScalarParameterValue (Variables|Default|GetMaterial) "EyePhaseNr" 32.0 :!class /Script/Engine.MaterialInstanceDynamic)
    (Utilities|FlowControl|Delay (Variables|Default|GetBetweenAnimationDelay))
    (Rendering|Material|SetScalarParameterValue (Variables|Default|GetMaterial) "EyePhaseNr" 33.0 :!class /Script/Engine.MaterialInstanceDynamic)
    (Utilities|FlowControl|Delay (Variables|Default|GetBetweenAnimationDelay))
    (Rendering|Material|SetScalarParameterValue (Variables|Default|GetMaterial) "EyePhaseNr" 27.0 :!class /Script/Engine.MaterialInstanceDynamic)
    (Utilities|FlowControl|Delay (Variables|Default|GetBetweenAnimationDelay))
    (Rendering|Material|SetScalarParameterValue (Variables|Default|GetMaterial) "EyePhaseNr" 28.0 :!class /Script/Engine.MaterialInstanceDynamic)
    (Utilities|FlowControl|Delay (Variables|Default|GetBetweenAnimationDelay))
    (Rendering|Material|SetScalarParameterValue (Variables|Default|GetMaterial) "EyePhaseNr" 29.0 :!class /Script/Engine.MaterialInstanceDynamic)
    (Utilities|FlowControl|Delay 1e+01)
    (CallFunction|EventSettoNeutral)
    (Variables|Default|SetCurrentlyChangingExpression false)))

(event EventBeginPlay)

(event Collision|EventActorBeginOverlap
  (params (OtherActor :type Actor%20Object%20Reference)))

(event EventTick
  (params (DeltaSeconds :type Float%20%28single-precision%29)))

(fn ConstructionScript
  (bind _returnvalue (Rendering|Material|CreateDynamicMaterialInstance (Variables|Default|GetStaticMesh) 0 "/Game/Character/NPC/M_RobotEyes.M_RobotEyes" "None" :!class /Script/Engine.PrimitiveComponent))
  (Rendering|Material|SetScalarParameterValue _returnvalue "EyePhaseNr" 0.0 :!class /Script/Engine.MaterialInstanceDynamic)
  (Variables|Default|SetMaterial _returnvalue))

(fn AdvanceEye
  (bind _material (Variables|Default|GetMaterial))
  (bind _returnvalue (Rendering|Material|GetScalarParameterValue _material "EyePhaseNr" :!class /Script/Engine.MaterialInstanceDynamic))
  (bind _result (Math|Float|IncrementFloat _returnvalue)
    (:%20%20
      (Rendering|Material|SetScalarParameterValue _material "EyePhaseNr" _result :!class /Script/Engine.MaterialInstanceDynamic))))