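; ShowOffRobot is an NPC robot character with a numbered widget, tinted armlet and expressive child-actor eyes that carries materials and wares.
; Timelines scale carried items' relative locations for drop and head-throw motions, while drop-off hands wares to a grabber.
; Expressions chain through randomly delayed self-calls, sometimes reflecting the LFB influence strategy, alongside a waving greeting.
; Triggered disobedience randomly chooses between no effect, slowed walking, stuttering speed or repeated idling.
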(event Custom|Cycle%20Random%20Expressions
  (bind _asbp_robot_eye (Utilities|Casting|CastToBP_RobotEye (Variables|/Script/Engine.ChildActorComponent|GetChildActor (Variables|Default|GetEyeL))))
  (bind _asbp_robot_eye_2 (Utilities|Casting|CastToBP_RobotEye (Variables|/Script/Engine.ChildActorComponent|GetChildActor (Variables|Default|GetEyeR))))
  (switch int (Math|Random|RandomIntegerinRange 0 11)
    (:3
      (Default|EventPlayHappy _asbp_robot_eye)
      (Default|EventPlayHappy _asbp_robot_eye_2))
    (:4
      (Default|EventBlink _asbp_robot_eye :!label _label)
      (Default|EventBlink _asbp_robot_eye_2))
    (:5
      (goto _label))
    (:6
      (goto _label))
    (:7
      (Default|EventSmallEyes _asbp_robot_eye :!label _label_2)
      (Default|EventSmallEyes _asbp_robot_eye_2))
    (:8
      (goto _label_2))
    (:9
      (Default|EventAngryEyeL _asbp_robot_eye)
      (Default|EventAngryEyeR _asbp_robot_eye_2))
    (:10
      (Default|EventSadEyes _asbp_robot_eye)
      (Default|EventSadEyes _asbp_robot_eye_2))
    (:11
      (Class|Robot|PlaySettingAppropriateExpression)))
  (Utilities|FlowControl|Delay (Math|Random|RandomFloatinRange 8.0 12.0))
  (CallFunction|CycleRandomExpressions))

(event EventBeginPlay
  (Variables|Default|SetMovementMaxSpeed (Class|MovementComponent|GetMaxSpeed (Variables|Character|GetCharacterMovement)))
  (bind _aswbp_robot_nr (Utilities|Casting|CastToWBP_RobotNr (UserInterface|GetUserWidgetObject (Variables|Default|GetWidget))))
  (Default|EventSetNr _aswbp_robot_nr (Class|Robot|GetRobotNr))
  (CallFunction|CycleRandomExpressions))

(event Collision|EventActorBeginOverlap
  (params (OtherActor :type Actor%20Object%20Reference)))

(event EventTick
  (params (DeltaSeconds :type Float%20%28single-precision%29)))

(event EventDropMaterialDown
  (bind _returnvalue (Class|Robot|GetCarriedMaterial))
  (bind _rootcomponent (Variables|/Script/Engine.Actor|GetRootComponent _returnvalue))
  (bind _returnvalue_2 (Transformation|GetRelativeTransform _rootcomponent))
  (bind _distancepercent (Timeline|Timeline_MaterialDrop PlayFromStart)
    (:Update
      (Transformation|SetActorRelativeTransform _returnvalue (Math|Transform|MakeTransform (* (.location _returnvalue_2) _distancepercent) (.rotation _returnvalue_2) (.scale _returnvalue_2)) false false))))

(event EventThrowWareonHead
  (bind _returnvalue (Class|Robot|GetCarriedWare))
  (bind _returnvalue_2 (Class|Robot|GetCarriedWare))
  (bind _rootcomponent (Variables|/Script/Engine.Actor|GetRootComponent _returnvalue))
  (bind _returnvalue_3 (Transformation|GetRelativeTransform _rootcomponent))
  (Transformation|AttachComponentToComponent (Class|Robot|GetCarriedWare) (Variables|Character|GetMesh) "CarrySocket" "KeepWorld" "KeepWorld" "KeepWorld" true)
  (bind (_direction _xdistance_ _ydistance_ _zdistance_) (Timeline|Timeline_WareThrow PlayFromStart)
    (:Update
      (Utilities|IsValid _returnvalue_2
        (:Is%20Valid
          (Transformation|SetActorRelativeTransform _returnvalue_2 (Math|Transform|MakeTransform (Math|Vector|MakeVector (* _xdistance_ (.x (.location _returnvalue_3))) (* _ydistance_ (.y (.location _returnvalue_3))) (* _zdistance_ (.z (.location _returnvalue_3)))) (.rotation _returnvalue_3) (.scale _returnvalue_3)) false false))))))

(event EventDropOffWare
  (params (WareGrabber :type Ware%20Grabber%20Object%20Reference))
  (Class|WareGrabber|MoveLowerPartUpandDown WareGrabber (Class|Robot|GetCarriedWare)))

(event EventActivateDisobedience
  (bind _returnvalue (Math|Random|RandomIntegerinRange 1 100))
  (if (not (Variables|Default|GetIsDisobedient))
    (Variables|Default|SetIsDisobedient true)
    (if (<= _returnvalue 25)
      _
      (elif (<= _returnvalue 50)
        (Variables|/Script/Engine.CharacterMovementComponent|SetMaxWalkSpeed (Variables|Character|GetCharacterMovement) (/ (Variables|Default|GetMovementMaxSpeed) 2.0))
        (Utilities|FlowControl|Delay 3e+01)
        (Variables|/Script/Engine.CharacterMovementComponent|SetMaxWalkSpeed (Variables|Character|GetCharacterMovement) (Variables|Default|GetMovementMaxSpeed))
        (elif (<= _returnvalue 75)
          (for _index (range 0 3)
            (Utilities|FlowControl|Delay 5.0)
            (Variables|/Script/Engine.CharacterMovementComponent|SetMaxWalkSpeed (Variables|Character|GetCharacterMovement) 1e+01)
            (Utilities|FlowControl|Delay 5.0)
            (Variables|/Script/Engine.CharacterMovementComponent|SetMaxWalkSpeed (Variables|Character|GetCharacterMovement) (Variables|Default|GetMovementMaxSpeed)))
          (else
            (for _index_2 (range 0 4)
              (Class|Robot|SetIdling)
              (Utilities|FlowControl|Delay 5.0))))))
    (Variables|Default|SetIsDisobedient false)))

(event EventPlayHappyGreeting
  (bind _mesh (Variables|Character|GetMesh))
  (Components|Animation|PlayAnimation _mesh "/Game/Character/NPC/Animations/Robot_Anim_Armature_Wave.Robot_Anim_Armature_Wave" false)
  (bind _asbp_robot_eye (Utilities|Casting|CastToBP_RobotEye (Variables|/Script/Engine.ChildActorComponent|GetChildActor (Variables|Default|GetEyeL))))
  (Default|EventPlayHappy _asbp_robot_eye)
  (bind _asbp_robot_eye_2 (Utilities|Casting|CastToBP_RobotEye (Variables|/Script/Engine.ChildActorComponent|GetChildActor (Variables|Default|GetEyeR))))
  (Default|EventPlayHappy _asbp_robot_eye_2)
  (Utilities|FlowControl|Delay 1.8)
  (Components|Animation|SetAnimationMode _mesh "AnimationBlueprint"))

(event EventPlaySettingAppropriateExpression
  (bind _eyel (Variables|Default|GetEyeL))
  (bind _eyer (Variables|Default|GetEyeR))
  (bind _childactor (Variables|/Script/Engine.ChildActorComponent|GetChildActor _eyel))
  (bind _childactor_2 (Variables|/Script/Engine.ChildActorComponent|GetChildActor _eyer))
  (bind _returnvalue (Class|WeinhoferLFBSettings|GetWeinhoferLFBSettings))
  (if (Math|Random|RandomBoolwithWeight 0.4)
    (switch Utilities|FlowControl|Switch|SwitchonEInfluenceStrategy (Class|WeinhoferLFBSettings|GetInfluenceStrategy _returnvalue)
      (:Emotion
        (bind _asbp_robot_eye (Utilities|Casting|CastToBP_RobotEye _childactor))
        (Default|EventPlayHappy _asbp_robot_eye)
        (bind _asbp_robot_eye_2 (Utilities|Casting|CastToBP_RobotEye _childactor_2))
        (Default|EventPlayHappy _asbp_robot_eye_2))
      (:Obstruction
        (bind _asbp_robot_eye_3 (Utilities|Casting|CastToBP_RobotEye _childactor))
        (Default|EventAngryEyeL _asbp_robot_eye_3)
        (bind _asbp_robot_eye_4 (Utilities|Casting|CastToBP_RobotEye _childactor_2))
        (Default|EventAngryEyeR _asbp_robot_eye_4)))))

(fn ConstructionScript
  (bind _returnvalue (Rendering|Material|CreateDynamicMaterialInstance (Variables|Default|GetArmlet) 0 "/Game/Character/NPC/Mesh/M_Armlet.M_Armlet" "None" :!class /Script/Engine.PrimitiveComponent))
  (Rendering|Material|SetVectorParameterValue _returnvalue "Color" (Variables|Default|GetArmletColor) :!class /Script/Engine.MaterialInstanceDynamic))