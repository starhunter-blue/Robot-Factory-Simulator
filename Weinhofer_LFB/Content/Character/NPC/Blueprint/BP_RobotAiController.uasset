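; AI controller for robot NPCs that runs the Robot_Behavior tree and mirrors robot state into its blackboard.
; On a state update it cancels any collect command, resets carried items, lift and office status, then writes the new state, work machine, dispenser and grabber keys.
; Office permission events toggle entry and route the permitted robot to its lift waypoint.
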(event EventBeginPlay
  (bind _blackboardcomponent (Class|AIController|UseBlackboard "/Game/Character/NPC/Blueprint/AI/Robot_BehaviorData.Robot_BehaviorData"))
  (Variables|Default|SetBlackboardComponent _blackboardcomponent)
  (AI|RunBehaviorTree "/Game/Character/NPC/Blueprint/AI/Robot_Behavior.Robot_Behavior"))

(event EventTick
  (params (DeltaSeconds :type Float%20%28single-precision%29)))

(event EventOnStateUpdated
  (Class|RobotAIController|TerminateCollectCommand)
  (bind _asbp_robot (Utilities|Casting|CastToBP_Robot (Pawn|GetControlledPawn)))
  (Class|Robot|DestroyCarriedStuff _asbp_robot)
  (Class|Robot|LeaveLift _asbp_robot)
  (Class|Robot|SetHasNotBeeninOffice _asbp_robot)
  (AI|Components|Blackboard|SetValueasEnum (Variables|Default|GetBlackboardComponent) (Variables|Default|GetRobotBehaviorState) (Class|RobotAIController|GetCurrentState))
  (AI|Components|Blackboard|SetValueasObject (Variables|Default|GetBlackboardComponent) (Variables|Default|GetTargetMachine) (Class|RobotAIController|GetWorkTargetMachine))
  (AI|Components|Blackboard|SetValueasObject (Variables|Default|GetBlackboardComponent) (Variables|Default|GetMaterialDispenserKey) (Class|RobotAIController|GetMaterialDispenser))
  (AI|Components|Blackboard|SetValueasObject (Variables|Default|GetBlackboardComponent) (Variables|Default|GetWareGrabberKey) (Class|RobotAIController|GetWareGrabber))
  (AI|Components|Blackboard|SetValueasBool (Variables|Default|GetBlackboardComponent) (Variables|Default|GetEnterOfficePermission) false)
  (AI|Components|Blackboard|ClearValue (Variables|Default|GetBlackboardComponent) (Variables|Default|GetDoorQueueSlotKey)))

(event EventPermittoEnterOffice
  (bind _asbp_robot (Utilities|Casting|CastToBP_Robot (Pawn|GetControlledPawn)))
  (Class|Robot|SetHasBeeninOffice _asbp_robot)
  (AI|Components|Blackboard|SetValueasObject (Variables|Default|GetBlackboardComponent) (Variables|Default|GetTargetWaypoint) (Class|Lift|GetLiftWaypoint (Class|Robot|GetLift _asbp_robot)))
  (AI|Components|Blackboard|SetValueasBool (Variables|Default|GetBlackboardComponent) (Variables|Default|GetEnterOfficePermission) true))

(event EventLeaveOffice
  (AI|Components|Blackboard|SetValueasBool (Variables|Default|GetBlackboardComponent) (Variables|Default|GetEnterOfficePermission) false))

(fn ConstructionScript)