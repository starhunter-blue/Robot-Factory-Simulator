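; Game mode for a timed factory task that tracks pyramid, cube and dodecahedron counts against targets from the Weinhofer LFB settings.
; On begin it configures the workscreen and the robot overlord's emotion or obstruction behavior, then pauses until StartActualPlay.
; A one-second looping timer updates the screen's remaining time, starts the overlord once at halftime, and at zero triggers the gameplay stopper and pauses again.
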(event Custom|Add1Pyramid
  (bind _result (Math|Integer|IncrementInt (Variables|Default|GetCurrentPyramidNr))
    (:%20%20
      (Default|SetPyramidHas (Variables|Default|GetWorkscreen) _result))))

(event Custom|Add1Cube
  (bind _result (Math|Integer|IncrementInt (Variables|Default|GetCurrentCubeNr))
    (:%20%20
      (Default|SetCubeHas (Variables|Default|GetWorkscreen) _result))))

(event Custom|Add1Dodecahedron
  (bind _result (Math|Integer|IncrementInt (Variables|Default|GetCurrentDodecahedronNr))
    (:%20%20
      (Default|SetDodecahedronHas (Variables|Default|GetWorkscreen) _result))))

(event Custom|Event%20Halftime
  (Class|RobotOverlord|Start (Variables|Default|GetOverlordReference)))

(event Custom|Event%20StartActualPlay
  (Game|SetGamePaused false)
  (Utilities|Time|SetTimerbyFunctionName 0 "DecreaseTimeBy1SecondAndInformWorkscreen" 1.0 true))

(event Custom|Event%20End%20Game
  (bind _outactors (Actor|GetAllActorsOfClass "/Game/UI/Factory/BP_GameplayStopper.BP_GameplayStopper_C"))
  (Default|EventStopGameplay (Utilities|Array|Get(acopy) _outactors))
  (Utilities|FlowControl|Delay 1.5)
  (Game|SetGamePaused true))

(event EventBeginPlay
  (bind _returnvalue (Class|WeinhoferLFBSettings|GetWeinhoferLFBSettings))
  (bind _output_get (Variables|Default|SetTimeLimitMinutes (Class|WeinhoferLFBSettings|GetTimeLimit _returnvalue)))
  (Variables|Default|SetTimeLeftSeconds (* _output_get 60))
  (Variables|Default|SetTargetPyramidNr (Class|WeinhoferLFBSettings|GetNrOfRequiredTriangles _returnvalue))
  (Variables|Default|SetTargetCubeNr (Class|WeinhoferLFBSettings|GetNrOfRequiredSquares _returnvalue))
  (Variables|Default|SetTargetDodecahedronNr (Class|WeinhoferLFBSettings|GetNrOfRequiredHexagons _returnvalue))
  (bind _outactors (Actor|GetAllActorsOfClass "/Game/Maps/Factory/Office/Blueprints/BP_Workscreen.BP_Workscreen_C"))
  (bind _output_get_2 (Variables|Default|SetWorkscreen (Utilities|Array|Get(acopy) _outactors)))
  (Default|SetPyramidShould _output_get_2 (Variables|Default|GetTargetPyramidNr))
  (Default|SetCubeShould _output_get_2 (Variables|Default|GetTargetCubeNr))
  (Default|SetDodecahedronShould _output_get_2 (Variables|Default|GetTargetDodecahedronNr))
  (bind _outactors_2 (Actor|GetAllActorsOfClass "/Game/Maps/Factory/BP_RobotOverlord.BP_RobotOverlord_C"))
  (bind _output_get_3 (Variables|Default|SetOverlordReference (Utilities|Array|Get(acopy) _outactors_2)))
  (switch Utilities|FlowControl|Switch|SwitchonEInfluenceStrategy (Class|WeinhoferLFBSettings|GetInfluenceStrategy _returnvalue)
    (:Emotion
      (Class|RobotOverlord|SetBehaviorTypetoEmotion _output_get_3))
    (:Obstruction
      (Class|RobotOverlord|SetBehaviorTypetoBlocking _output_get_3)))
  (Utilities|FlowControl|Delay 0.5)
  (Game|SetGamePaused true))

(event EventTick
  (params (DeltaSeconds :type Float%20%28single-precision%29)))

(fn ConstructionScript)

(fn DecreaseTimeby1SecondandInformWorkscreen
  (bind _result (Math|Integer|DecrementInt (Variables|Default|GetTimeLeftSeconds))
    (:%20%20
      (Default|UpdateTimePercentLeft (Variables|Default|GetWorkscreen) (/ (Math|Conversions|ToFloat(Integer) _result) (* (Variables|Default|GetTimeLimitMinutes) 6e+01)))
      (if (<= (/ (Math|Conversions|ToFloat(Integer) _result) (* (Variables|Default|GetTimeLimitMinutes) 6e+01)) 0.0)
        (CallFunction|EventEndGame)
        (elif (and (<= (/ (Math|Conversions|ToFloat(Integer) _result) (* (Variables|Default|GetTimeLimitMinutes) 6e+01)) 0.5) (Variables|Default|GetHalfTimeNotTriggered))
          (Variables|Default|SetHalfTimeNotTriggered false)
          (CallFunction|EventHalftime))))))