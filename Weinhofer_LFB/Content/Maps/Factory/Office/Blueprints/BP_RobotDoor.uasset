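; BP_RobotDoor is an automatic sliding door with red and green status lamps, placed in the Factory Office map.
; Its trigger volume opens the door on any begin overlap and closes it on end overlap, without filtering actors or counting occupants.
; Separate open and close timelines drive the door's relative Z from the start on each call.
; The construction script creates dynamic lamp materials, whose "Light On" parameter switches between green when opening and red when closing.
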(event Custom|OnTriggerVolumeOverlap
  (params (OverlappedComponent :type Primitive%20Component%20Object%20Reference) (OtherActor :type Actor%20Object%20Reference) (OtherComp :type Primitive%20Component%20Object%20Reference) (OtherBodyIndex :type Integer) (bFromSweep :type Boolean) (SweepResult :type Hit%20Result%20Structure%20%28by%20ref%29))
  (Class|RobotDoor|OpenDoor))

(event Custom|OnTriggerVolumeEndOverlap
  (params (OverlappedComponent :type Primitive%20Component%20Object%20Reference) (OtherActor :type Actor%20Object%20Reference) (OtherComp :type Primitive%20Component%20Object%20Reference) (OtherBodyIndex :type Integer))
  (Class|RobotDoor|CloseDoor))

(event EventBeginPlay
  (Rendering|Material|SetScalarParameterValue (Variables|Default|GetRed%20Light%20Material) "Light On" 1.0 :!class /Script/Engine.MaterialInstanceDynamic)
  (Collision|AssignOnComponentBeginOverlap (Variables|Default|GetDoorOpenCloseTriggerVolume) (delegate Custom|OnTriggerVolumeOverlap))
  (Collision|AssignOnComponentEndOverlap (Variables|Default|GetDoorOpenCloseTriggerVolume) (delegate Custom|OnTriggerVolumeEndOverlap)))

(event EventTick
  (params (DeltaSeconds :type Float%20%28single-precision%29)))

(event EventOpenDoor
  (Rendering|Material|SetScalarParameterValue (Variables|Default|GetGreen%20Light%20Material) "Light On" 1.0 :!class /Script/Engine.MaterialInstanceDynamic)
  (Rendering|Material|SetScalarParameterValue (Variables|Default|GetRed%20Light%20Material) "Light On" 0.0 :!class /Script/Engine.MaterialInstanceDynamic)
  (bind _zlocation (Timeline|Timeline_OpenDoor PlayFromStart)
    (:Update
      (Transformation|SetRelativeLocation (Variables|Default|GetDoor) (Math|Vector|MakeVector 0.0 0.0 _zlocation) false false))))

(event EventCloseDoor
  (Rendering|Material|SetScalarParameterValue (Variables|Default|GetGreen%20Light%20Material) "Light On" 0.0 :!class /Script/Engine.MaterialInstanceDynamic)
  (Rendering|Material|SetScalarParameterValue (Variables|Default|GetRed%20Light%20Material) "Light On" 1.0 :!class /Script/Engine.MaterialInstanceDynamic)
  (bind _zlocation (Timeline|Timeline_CloseDoor PlayFromStart)
    (:Update
      (Transformation|SetRelativeLocation (Variables|Default|GetDoor) (Math|Vector|MakeVector 0.0 0.0 _zlocation) false false))))

(fn ConstructionScript
  (bind _returnvalue (Rendering|Material|CreateDynamicMaterialInstance (Variables|Default|GetRed%20Light) 0 "/Game/Maps/Factory/Office/Meshes/RobotDoor/MI_RedLamp.MI_RedLamp" "None" :!class /Script/Engine.PrimitiveComponent))
  (Variables|Default|SetRed%20Light%20Material _returnvalue)
  (bind _returnvalue_2 (Rendering|Material|CreateDynamicMaterialInstance (Variables|Default|GetGreen%20Light) 0 "/Game/Maps/Factory/Office/Meshes/RobotDoor/MI_GreenLamp.MI_GreenLamp" "None" :!class /Script/Engine.PrimitiveComponent))
  (Variables|Default|SetGreen%20Light%20Material _returnvalue_2))