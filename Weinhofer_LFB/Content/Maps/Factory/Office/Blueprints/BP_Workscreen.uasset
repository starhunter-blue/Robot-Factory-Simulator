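; Office workscreen actor in the factory map that bridges its WBP_Workscreen widget and the robot management game logic.
; On BeginPlay it binds to the widget's order events and relays production, supply, collect and office call, let-in or dismiss requests outward.
; Let-in requests check for a queued robot, otherwise resetting the button.
; Incoming events push robot agendas, current and target shape counts, remaining time and office departures to the widget.
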(event Custom|Event%20Send%20Production%20Order
  (params (TargetRobotNr :type Integer) (WareType :type EWareType%20Enum :default "WTE_UNSET"))
  (Class|Workscreen|SendProductionOrder TargetRobotNr WareType))

(event Custom|SetPyramidShould
  (params (Nr :type Integer))
  ;[1 1 1] Update First Page of Screen
  (bind _aswbp_workscreen (Utilities|Casting|CastToWBP_Workscreen (UserInterface|GetUserWidgetObject (Variables|Default|GetWidget))))
  (Default|SetPyramidShould _aswbp_workscreen Nr))

(event Custom|SetDodecahedronHas
  (params (Nr :type Integer))
  ;[1 1 1] Update First Page of Screen
  (bind _aswbp_workscreen (Utilities|Casting|CastToWBP_Workscreen (UserInterface|GetUserWidgetObject (Variables|Default|GetWidget))))
  (Default|SetDodecahedronHas _aswbp_workscreen Nr))

(event Custom|Send%20Let%20Into%20Office
  (if (Class|Workscreen|QueueHasRobot)
    (Class|Workscreen|LetRobotIntoOffice)
    (else
      (bind _aswbp_workscreen (Utilities|Casting|CastToWBP_Workscreen (UserInterface|GetUserWidgetObject (Variables|Default|GetWidget))))
      (Default|SetLetIn/DismissRobotButtontoDefault _aswbp_workscreen))))

(event Custom|Send%20Dismiss%20From%20Office
  (Class|Workscreen|DismissRobotfromOffice))

(event Custom|SetDodecahedronShould
  (params (Nr :type Integer))
  ;[1 1 1] Update First Page of Screen
  (bind _aswbp_workscreen (Utilities|Casting|CastToWBP_Workscreen (UserInterface|GetUserWidgetObject (Variables|Default|GetWidget))))
  (Default|SetDodecahedronShould _aswbp_workscreen Nr))

(event Custom|Event%20Send%20Collect%20Order
  (params (Target%20Robot%20Nr :type Integer))
  (Class|Workscreen|SendCollectOrder Target%20Robot%20Nr))

(event Custom|SetPyramidHas
  (params (Nr :type Integer))
  ;[1 1 1] Update First Page of Screen
  (bind _aswbp_workscreen (Utilities|Casting|CastToWBP_Workscreen (UserInterface|GetUserWidgetObject (Variables|Default|GetWidget))))
  (Default|SetPyramidHas _aswbp_workscreen Nr))

(event Custom|Event%20Send%20Supply%20Order
  (params (TargetMachine :type BP%20Machine%20Object%20Reference) (TargetRobotNr :type Integer))
  (Class|Workscreen|SendSupplyOrder TargetRobotNr TargetMachine))

(event Custom|SetCubeHas
  (params (Nr :type Integer))
  ;[1 1 1] Update First Page of Screen
  (bind _aswbp_workscreen (Utilities|Casting|CastToWBP_Workscreen (UserInterface|GetUserWidgetObject (Variables|Default|GetWidget))))
  (Default|SetCubeHas _aswbp_workscreen Nr))

(event Custom|UpdateTimePercentLeft
  (params (Percent :type Float%20%28single-precision%29))
  ;[1 1 1] Update First Page of Screen
  (bind _aswbp_workscreen (Utilities|Casting|CastToWBP_Workscreen (UserInterface|GetUserWidgetObject (Variables|Default|GetWidget))))
  (Default|UpdateTimePercent _aswbp_workscreen Percent))

(event Custom|SetCubeShould
  (params (Nr :type Integer))
  ;[1 1 1] Update First Page of Screen
  (bind _aswbp_workscreen (Utilities|Casting|CastToWBP_Workscreen (UserInterface|GetUserWidgetObject (Variables|Default|GetWidget))))
  (Default|SetCubeShould _aswbp_workscreen Nr))

(event Custom|Send%20Call%20To%20Office%20Order
  (params (TargetRobotNr :type Integer))
  (Class|Workscreen|SendCalltoOfficeOrder TargetRobotNr))

(event EventBeginPlay
  (bind _aswbp_workscreen (Utilities|Casting|CastToWBP_Workscreen (UserInterface|GetUserWidgetObject (Variables|Default|GetWidget))))
  (EventDispatchers|BindEventtoRobotMachineWorkOrder _aswbp_workscreen (delegate Custom|Event%20Send%20Production%20Order))
  (EventDispatchers|BindEventtoRobotSupplyWorkOrder _aswbp_workscreen (delegate Custom|Event%20Send%20Supply%20Order))
  (EventDispatchers|BindEventtoRobotCollectWorkOrder _aswbp_workscreen (delegate Custom|Event%20Send%20Collect%20Order))
  (EventDispatchers|BindEventtoRobotCalltoOfficeOrder _aswbp_workscreen (delegate Custom|Send%20Call%20To%20Office%20Order))
  (EventDispatchers|BindEventtoRobotLetIntoOffice _aswbp_workscreen (delegate Custom|Send%20Let%20Into%20Office))
  (EventDispatchers|BindEventtoRobotDismissfromOffice _aswbp_workscreen (delegate Custom|Send%20Dismiss%20From%20Office)))

(event Collision|EventActorBeginOverlap
  (params (OtherActor :type Actor%20Object%20Reference)))

(event EventTick
  (params (DeltaSeconds :type Float%20%28single-precision%29)))

(event EventInformOfRoboterLeavingOffice
  (bind _aswbp_workscreen (Utilities|Casting|CastToWBP_Workscreen (UserInterface|GetUserWidgetObject (Variables|Default|GetWidget))))
  (Default|SetLetIn/DismissRobotButtontoDefault _aswbp_workscreen)
  (Default|RemoveRobotAgenda _aswbp_workscreen))

(event EventGiveRobotAgenda
  (params (RobotNr :type Integer) (RobotAgenda :type Robot%20Agenda%20Object%20Reference))
  (bind _aswbp_workscreen (Utilities|Casting|CastToWBP_Workscreen (UserInterface|GetUserWidgetObject (Variables|Default|GetWidget))))
  (Default|GiveRobotAgenda _aswbp_workscreen RobotNr RobotAgenda))

(fn ConstructionScript)