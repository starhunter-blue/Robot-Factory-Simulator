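; BP_Machine is a factory machine that turns material into wares and shows its production state on a progress bar widget.
; The widget switches between progress, ready-to-collect and no-material screens.
; SpawnWare consumes one material, spawns a ware at a mesh socket and animates it out on a timeline-driven mover before detaching it.
; A retriggerable 90-second delay then destroys any still-valid current ware and clears the collect flag.
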(event Custom|Event%20Destroy%20Stuck%20Ware
  (bind _returnvalue (Class|Machine|GetCurrentWare))
  (Utilities|FlowControl|RetriggerableDelay 9e+01)
  (Utilities|IsValid _returnvalue
    (:Is%20Valid
      (Actor|DestroyActor _returnvalue)
      (Class|Machine|SetWaretoCollect false))))

(event EventSetProgressBar
  (bind _progressbar (Variables|Default|GetProgressBar))
  (bind _returnvalue (UserInterface|GetUserWidgetObject _progressbar))
  (if (Class|Machine|HasMaterial)
    (if (Class|Machine|IsWaretoCollect)
      (bind _aswbp_machine_progress_bar (Utilities|Casting|CastToWBP_MachineProgressBar _returnvalue))
      (Default|SetScreentoCollectWare _aswbp_machine_progress_bar)
      (else
        (bind _aswbp_machine_progress_bar_2 (Utilities|Casting|CastToWBP_MachineProgressBar _returnvalue))
        (Default|SetProgressBar _aswbp_machine_progress_bar_2 (Class|Machine|GetProductionProgress))
        (Default|SetScreentoNormal _aswbp_machine_progress_bar_2)))
    (else
      (bind _aswbp_machine_progress_bar_3 (Utilities|Casting|CastToWBP_MachineProgressBar _returnvalue))
      (Default|SetScreentoNoMaterial _aswbp_machine_progress_bar_3))))

(event EventSpawnWare
  (bind _waremover (Variables|Default|GetWareMover))
  (if (Class|Machine|HasMaterial)
    (Class|Machine|SetWaretoCollect true)
    (Class|Machine|UseOneMaterial)
    (bind _returnvalue (Game|SpawnActorfromClass (Class|Machine|GetWareClass) (Math|Conversions|ToTransform(Vector) (Transformation|GetSocketLocation (Variables|Default|GetMachineBodyMesh) (Variables|Default|GetWareSpawnpoint))) "Undefined" 0 0))
    (Class|Machine|SetCurrentWare _returnvalue)
    (Transformation|AttachComponentToComponent _returnvalue (Variables|Default|GetWareMover) "None" "SnapToTarget" "KeepRelative" "KeepRelative" true)
    (bind (_direction _rotation _location) (Timeline|Timeline_0 PlayFromStart)
      (:Update
        (Transformation|SetRelativeLocation _waremover _location false false)
        (Transformation|SetRelativeRotation _waremover (Math|Rotator|MakeRotator 0.0 _rotation 0.0) false false))
      (:Finished
        (Transformation|DetachFromActor _returnvalue "KeepWorld" "KeepRelative" "KeepRelative")
        (Transformation|SetRelativeLocation _waremover "0, 0, 0" false false)
        (Transformation|SetRelativeRotation _waremover "0, 0, 0" false false)
        (CallFunction|EventDestroyStuckWare)))))

(fn ConstructionScript)