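; BP_WareGrabber is a factory room grabber that moves its lower part vertically and drops off wares to be counted.
; MoveLowerPartUpandDown plays the Movement timeline, scaling its Z track by LowerPartRelativeZ to set the lower mesh's relative height.
; When an update finds the track value near zero, a valid ware increments its type's counter (Pyramid, Cube or Dodecahedron) on Factory_Mode_BP and is destroyed.
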(event EventBeginPlay)

(event Collision|EventActorBeginOverlap
  (params (OtherActor :type Actor%20Object%20Reference)))

(event EventTick
  (params (DeltaSeconds :type Float%20%28single-precision%29)))

(event EventMoveLowerPartUpandDown
  (params (WareToDropOff :type Actor%20Object%20Reference))
  (bind _waregrabberlowermesh (Variables|Default|GetWareGrabberLowerMesh))
  (bind _returnvalue (Transformation|GetRelativeTransform _waregrabberlowermesh))
  (bind _z_ (Timeline|Movement PlayFromStart)
    (:Update
      (Transformation|SetRelativeLocation (Variables|Default|GetWareGrabberLowerMesh) (Math|Vector|MakeVector (.x (.location _returnvalue)) (.y (.location _returnvalue)) (* _z_ (Variables|Default|GetLowerPartRelativeZ))) false false)
      (if (Math|Float|NearlyEqual(Float) _z_ 0.0 0.0001)
        (Utilities|IsValid WareToDropOff
          (:Is%20Valid
            (bind _asware (Utilities|Casting|CastToWare WareToDropOff))
            (bind _asfactory_mode_bp (Utilities|Casting|CastToFactory_Mode_BP (Game|GetGameMode)))
            (switch Utilities|FlowControl|Switch|SwitchonEWareType (Class|Ware|GetWareType _asware)
              (:WTE_UNSET
                _)
              (:WTE_Pyramid
                (Default|Add1Pyramid _asfactory_mode_bp))
              (:WTE_Cube
                (Default|Add1Cube _asfactory_mode_bp))
              (:WTE_Dodecahedron
                (Default|Add1Dodecahedron _asfactory_mode_bp)))
            (Actor|DestroyActor WareToDropOff)))))))

(fn ConstructionScript)